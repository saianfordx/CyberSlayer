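; Bullet actor that flies at the player character, damages it and explodes.
; On BeginPlay it caches the direction and look-at rotation toward MyCharacter, so it does not home.
; Each tick it moves MainSprite along that line by Speed, then runs a debug-drawn sphere trace at the actor location.
; A hit whose display name is "MyCharacter" applies Damage, spawns Explotion_01_BP and destroys the bullet.
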(event `self.ReceiveBeginPlay`
  (bind _targetpoint (`self.getTargetPoint`))
  (set `self.impactPoint` _targetpoint)
  (bind _targetrotationpoint (`self.lookAt`))
  (set `self.rotation` _targetrotationpoint))

(event `self.ReceiveTick`
  (params (DeltaSeconds :type "Float (single-precision)"))
  (bind _transform (`self.shoot` (`self.impactPoint`) (`self.rotation`)))
  (`SceneComponent.K2_SetWorldTransform` (`self.MainSprite`) _transform false false)
  (`self.Apply Damage`))

(fn `Apply Damage`
  (bind _returnvalue (`self.K2_GetActorLocation`))
  (bind _outhits (`KismetSystemLibrary.SphereTraceMulti` :`Start` _returnvalue :`End` _returnvalue :`Radius` 30.0 :`TraceChannel` "TraceTypeQuery1" :`DrawDebugType` "ForOneFrame"))
  (for _array_element _outhits
    (if (`KismetStringLibrary.EqualEqual_StrStr` (`KismetSystemLibrary.GetDisplayName` (`.HitActor` (`GameplayStatics.BreakHitResult` _array_element))) "MyCharacter")
      (bind _returnvalue_2 (`GameplayStatics.GetActorOfClass` "/Game/Logical_And_/Blueprints/Actors/Player/MyCharacter.MyCharacter_C"))
      (`GameplayStatics.ApplyDamage` _returnvalue_2 (`self.Damage`))
      (`|SpawnActorFromClass` "/Game/Logical_And_/Blueprints/Animations/Explotions/Explotion_01/Explotion_01_BP.Explotion_01_BP_C" (`self.GetTransform`) "Undefined" "OverrideRootScale" null null)
      (`self.K2_DestroyActor`))))

(fn `getTargetPoint`
  (returns (TargetPoint :type "Vector Structure"))
  (bind _returnvalue (`GameplayStatics.GetActorOfClass` "/Game/Logical_And_/Blueprints/Actors/Player/MyCharacter.MyCharacter_C"))
  (return (`KismetMathLibrary.Normal` (- (`self.K2_GetActorLocation` _returnvalue) (`SceneComponent.K2_GetComponentLocation` (`self.MainSprite`))))))

(fn `lookAt`
  (returns (TargetRotationPoint :type "Rotator Structure"))
  (bind _returnvalue (`GameplayStatics.GetActorOfClass` "/Game/Logical_And_/Blueprints/Actors/Player/MyCharacter.MyCharacter_C"))
  (bind (_returnvalue_roll _returnvalue_pitch _returnvalue_yaw) (`KismetMathLibrary.BreakRotator` (`KismetMathLibrary.FindLookAtRotation` (`SceneComponent.K2_GetComponentLocation` (`self.MainSprite`)) (`self.K2_GetActorLocation` _returnvalue))))
  (return (`KismetMathLibrary.MakeRotator` _returnvalue_roll _returnvalue_pitch _returnvalue_yaw)))

(fn `shoot`
  (params (targetHit :type "Vector Structure") (targetRotation :type "Rotator Structure"))
  (returns (transform :type "Transform Structure"))
  (return (`KismetMathLibrary.MakeTransform` (+ (`SceneComponent.K2_GetComponentLocation` (`self.MainSprite`)) (* targetHit (* (`self.speed`) (`GameplayStatics.GetWorldDeltaSeconds`)))) targetRotation (`SceneComponent.K2_GetComponentScale` (`self.MainSprite`)))))

(fn `UserConstructionScript`)