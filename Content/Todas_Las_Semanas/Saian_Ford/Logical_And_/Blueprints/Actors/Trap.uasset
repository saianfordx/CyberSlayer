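; Trap actor that shows a flipbook animation and damages the player character when it comes within a small radius.
; Every tick it runs a sphere trace on the Visibility channel, with debug drawing, and matches hit actors by the display name "MyCharacter".
; A match applies Damage to the first MyCharacter found in the world and clears IsActive, which stops further checks only when IsOneTimeDamage is set.
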(event `self.ReceiveBeginPlay`
  (`PaperFlipbookComponent.SetFlipbook` (`self.Trap_FB`) (`self.Animation`)))

(event `self.ReceiveTick`
  (params (DeltaSeconds :type "Float (single-precision)"))
  (if (`self.isOneTimeDamage`)
    (if (`self.isActive`)
      (`self.detectPlayer`))
    (else
      (`self.detectPlayer`))))

(fn `detectPlayer`
  (bind _returnvalue (`self.K2_GetActorLocation`))
  (bind _outhits (`KismetSystemLibrary.SphereTraceMulti` :`Start` _returnvalue :`End` _returnvalue :`Radius` 30.0 :`TraceChannel` "TraceTypeQuery1" :`DrawDebugType` "ForOneFrame"))
  (for _array_element _outhits
    (if (`KismetStringLibrary.EqualEqual_StrStr` (`KismetSystemLibrary.GetDisplayName` (`.HitActor` (`GameplayStatics.BreakHitResult` _array_element))) "MyCharacter")
      (bind _returnvalue_2 (`GameplayStatics.GetActorOfClass` "/Game/Logical_And_/Blueprints/Actors/Player/MyCharacter.MyCharacter_C"))
      (`GameplayStatics.ApplyDamage` _returnvalue_2 (`self.Damage`))
      (set `self.isActive` false))))

(fn `UserConstructionScript`)