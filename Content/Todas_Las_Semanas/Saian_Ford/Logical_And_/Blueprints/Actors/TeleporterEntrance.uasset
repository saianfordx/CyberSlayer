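; TeleporterEntrance is an actor that moves the player character to a TeleporterExit in the level.
; Every Tick, its Teleport function runs a multi sphere trace in place on the Visibility channel, with debug drawing for one frame.
; Any hit actor whose display name is "MyCharacter" has its root component moved to the location of the TeleporterExit found by GetActorOfClass.
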(event `self.ReceiveTick`
  (params (DeltaSeconds :type "Float (single-precision)"))
  (`self.Teleport`))

(fn `Teleport`
  (bind _returnvalue (`self.K2_GetActorLocation`))
  (bind _outhits (`KismetSystemLibrary.SphereTraceMulti` :`Start` _returnvalue :`End` _returnvalue :`Radius` 100.0 :`TraceChannel` "TraceTypeQuery1" :`DrawDebugType` "ForOneFrame"))
  (for _array_element _outhits
    (bind (_bblockinghit _binitialoverlap _time _distance _location _impactpoint _normal _impactnormal _physmat _hitactor) (`GameplayStatics.BreakHitResult` _array_element))
    (if (`KismetStringLibrary.EqualEqual_StrStr` (`KismetSystemLibrary.GetDisplayName` _hitactor) "MyCharacter")
      (bind _returnvalue_2 (`GameplayStatics.GetActorOfClass` "/Game/Logical_And_/Blueprints/Actors/TeleporterExit.TeleporterExit_C"))
      (`SceneComponent.K2_SetWorldLocation` (`Actor.RootComponent` _hitactor) (`SceneComponent.K2_GetComponentLocation` (`Actor.RootComponent` _returnvalue_2)) false false))))

(fn `UserConstructionScript`)