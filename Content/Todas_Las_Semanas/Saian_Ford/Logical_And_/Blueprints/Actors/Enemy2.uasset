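; Paper2D robot enemy that patrols along the X axis and fires bullets at MyCharacter.
; Each Tick, a sphere trace latches detection, then a line trace to the player triggers Shoot; the trailing Delay does not throttle it.
; Otherwise it steps along X with swept moves, flipping direction through checks against its start X.
; The floor-trace Patrol, forward-only player detection and flipbook rotation helpers are unused.
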(event `self.ReceiveBeginPlay`
  (bind _returnvalue_x (`KismetMathLibrary.BreakVector` (`self.K2_GetActorLocation`)))
  (set `self.InitialPositionX` _returnvalue_x))

(event `self.ReceiveTick`
  (params (DeltaSeconds :type "Float (single-precision)"))
  (`self.Update Flipbook`)
  (`self.Listen`)
  (if (`self.isEnemyDetected`)
    (bind _isdetected (`self.DetectPlayerBack`))
    (if _isdetected
      (`self.Shoot`)
      (`KismetSystemLibrary.Delay` 4.0)
      (else
        (if (> (`self.direction`) 0.0) :!label _label
          (`self.PatrolByDistance`)
          (`self.WalkForward`)
          (else
            (`self.PatrolByDistance`)
            (`self.WalkBackwards`)))))
    (else
      (goto _label))))

(fn `AdjustDirection`
  (bind (_returnvalue_roll _returnvalue_pitch _returnvalue_yaw) (`KismetMathLibrary.BreakRotator` (`self.K2_GetActorRotation`)))
  (if (> (`self.direction`) 0.0)
    (set `self.direction` -1.0)
    (else
      (set `self.direction` 1.0)))
  (`self.K2_SetActorRotation` (`KismetMathLibrary.MakeRotator` 0.0 0.0 (+ 180.0 _returnvalue_yaw))))

(fn `AdjustFBDirection`
  (bind (_returnvalue_roll _returnvalue_pitch) (`KismetMathLibrary.BreakRotator` (`SceneComponent.K2_GetComponentRotation` (`self.PaperFlipbook`))))
  (bind _returnvalue (`GameplayStatics.GetActorOfClass` "/Game/Logical_And_/Blueprints/Actors/Player/MyCharacter.MyCharacter_C"))
  (bind (_returnvalue_x _returnvalue_y _returnvalue_z) (`KismetMathLibrary.BreakVector` (`SceneComponent.GetForwardVector` (`Actor.RootComponent` _returnvalue))))
  (`SceneComponent.K2_SetWorldRotation` (`self.PaperFlipbook`) (`KismetMathLibrary.MakeRotator` _returnvalue_x _returnvalue_pitch _returnvalue_z) false false))

(fn `DetectFloorBackward`
  (bind (_returnvalue_x _returnvalue_y _returnvalue_z) (`KismetMathLibrary.BreakVector` (`KismetMathLibrary.GetForwardVector` (`self.K2_GetActorRotation`))))
  (bind _outhit (`KismetSystemLibrary.LineTraceSingle` (`self.K2_GetActorLocation`) (`KismetMathLibrary.MakeVector` (+ _returnvalue_x -1200.0) _returnvalue_y _returnvalue_z) "TraceTypeQuery1"))
  (if (not (`KismetStringLibrary.EqualEqual_StrStr` (`KismetSystemLibrary.GetDisplayName` (`.HitActor` (`GameplayStatics.BreakHitResult` _outhit))) (`self.FloorName`)))
    (`self.AdjustDirection`)))

(fn `DetectFloorForward`
  (bind (_returnvalue_x _returnvalue_y _returnvalue_z) (`KismetMathLibrary.BreakVector` (`KismetMathLibrary.GetForwardVector` (`self.K2_GetActorRotation`))))
  (bind _outhit (`KismetSystemLibrary.LineTraceSingle` (`self.K2_GetActorLocation`) (`KismetMathLibrary.MakeVector` (+ _returnvalue_x 200.0) _returnvalue_y _returnvalue_z) "TraceTypeQuery1"))
  (if (not (`KismetStringLibrary.EqualEqual_StrStr` (`KismetSystemLibrary.GetDisplayName` (`.HitActor` (`GameplayStatics.BreakHitResult` _outhit))) (`self.FloorName`)))
    (`self.AdjustDirection`)))

(fn `DetectPlayer`
  (returns (isDetected :type Boolean))
  (bind _returnvalue (`self.K2_GetActorLocation`))
  (bind _outhit (`KismetSystemLibrary.LineTraceSingle` _returnvalue (+ _returnvalue (* (`KismetMathLibrary.GetForwardVector` (`self.K2_GetActorRotation`)) 350)) "TraceTypeQuery1"))
  (if (`KismetStringLibrary.EqualEqual_StrStr` "MyCharacter" (`KismetSystemLibrary.GetDisplayName` (`.HitActor` (`GameplayStatics.BreakHitResult` _outhit))))
    (set `self.Trace_Hiting` true)
    (return true)
    (else
      (set `self.Trace_Hiting` false)
      (return false))))

(fn `DetectPlayerBack`
  (returns (isDetected :type Boolean))
  (bind (_returnvalue_x _returnvalue_y _returnvalue_z) (`KismetMathLibrary.BreakVector` (`self.K2_GetActorLocation`)))
  (bind _returnvalue (`GameplayStatics.GetActorOfClass` "/Game/Logical_And_/Blueprints/Actors/Player/MyCharacter.MyCharacter_C"))
  (bind (_returnvalue_x_2 _returnvalue_y_2 _returnvalue_z_2) (`KismetMathLibrary.BreakVector` (`self.K2_GetActorLocation` _returnvalue)))
  (bind _outhit (`KismetSystemLibrary.LineTraceSingle` :`Start` (`KismetMathLibrary.MakeVector` _returnvalue_x _returnvalue_y _returnvalue_z) :`End` (`KismetMathLibrary.MakeVector` _returnvalue_x_2 _returnvalue_y_2 _returnvalue_z_2) :`TraceChannel` "TraceTypeQuery1" :`DrawDebugType` "ForOneFrame"))
  (if (`KismetStringLibrary.EqualEqual_StrStr` "MyCharacter" (`KismetSystemLibrary.GetDisplayName` (`.HitActor` (`GameplayStatics.BreakHitResult` _outhit))))
    (set `self.Trace_Hiting` true)
    (return true)
    (else
      (set `self.Trace_Hiting` false)
      (return false))))

(fn `Listen`
  (bind _returnvalue (`self.K2_GetActorLocation`))
  (bind _outhits (`KismetSystemLibrary.SphereTraceMulti` _returnvalue _returnvalue 500.0 "TraceTypeQuery1"))
  (for _array_element _outhits
    (if (`KismetStringLibrary.EqualEqual_StrStr` (`KismetSystemLibrary.GetDisplayName` (`.HitActor` (`GameplayStatics.BreakHitResult` _array_element))) "MyCharacter")
      (set `self.isEnemyDetected` true)
      (if (`self.Trace_Hiting`)
        _))))

(fn `Patrol`
  (`self.Listen`)
  (if (`self.isEnemyDetected`)
    (bind _isdetected (`self.DetectPlayer`))
    (if _isdetected
      (set `self.isShooting` true)
      (else
        (if (> (`self.direction`) 0.0) :!label _label
          (`self.DetectFloorForward`)
          (`self.WalkForward`)
          (else
            (`self.DetectFloorBackward`)
            (`self.WalkBackwards`)))))
    (else
      (goto _label))))

(fn `PatrolByDistance`
  (bind _returnvalue_x (`KismetMathLibrary.BreakVector` (`self.K2_GetActorLocation`)))
  (bind _returnvalue_x_2 (`KismetMathLibrary.BreakVector` (`self.K2_GetActorLocation`)))
  (if (> (`self.direction`) 0.0)
    (if (<= (- _returnvalue_x_2 (`self.InitialPositionX`)) 0.0)
      (`self.AdjustDirection`))
    (elif (>= (+ _returnvalue_x (`self.InitialPositionX`)) (`self.InitialPositionX`))
      (`self.AdjustDirection`))))

(fn `SetRotation`
  (bind (_returnvalue_roll _returnvalue_pitch) (`KismetMathLibrary.BreakRotator` (`SceneComponent.K2_GetComponentRotation` (`self.PaperFlipbook`))))
  (bind (_returnvalue_roll_2 _returnvalue_pitch_2) (`KismetMathLibrary.BreakRotator` (`SceneComponent.K2_GetComponentRotation` (`self.PaperFlipbook`))))
  (bind _velocity_x (`KismetMathLibrary.BreakVector` (`MovementComponent.Velocity` (`self.CharacterMovement`))))
  (if (< _velocity_x 0.0)
    (`SceneComponent.K2_SetWorldRotation` (`self.PaperFlipbook`) (`KismetMathLibrary.MakeRotator` _returnvalue_roll _returnvalue_pitch 180.0) false false)
    (elif (!= _velocity_x 0.0)
      (`SceneComponent.K2_SetWorldRotation` (`self.PaperFlipbook`) (`KismetMathLibrary.MakeRotator` _returnvalue_roll_2 _returnvalue_pitch_2) false false))))

(fn `Shoot`
  (`PaperFlipbookComponent.SetFlipbook` (`self.PaperFlipbook`) "/Game/Logical_And_/Blueprints/Animations/Robot/Robot_Shoot_FB.Robot_Shoot_FB")
  (`|SpawnActorFromClass` "/Game/Logical_And_/Blueprints/Actors/Bullet.Bullet_C" (`self.GetTransform`) "Undefined" "OverrideRootScale" null null))

(fn `Update Flipbook`
  (if true
    (if (> (`KismetMathLibrary.Abs` (`KismetMathLibrary.VSize` (`MovementComponent.Velocity` (`self.CharacterMovement`)))) 0.0)
      (`PaperFlipbookComponent.SetFlipbook` (`self.PaperFlipbook`) "/Game/Logical_And_/Blueprints/Animations/Robot/Robot_Shoot_FB.Robot_Shoot_FB")
      (else
        (`PaperFlipbookComponent.SetFlipbook` (`self.PaperFlipbook`) "/Game/Logical_And_/Blueprints/Animations/Robot/Robot_Run_FB.Robot_Run_FB")))))

(fn `UserConstructionScript`)

(fn `WalkBackwards`
  (bind (_returnvalue_x _returnvalue_y _returnvalue_z) (`KismetMathLibrary.BreakVector` (`self.K2_GetActorLocation`)))
  (`self.K2_SetActorLocation` (`KismetMathLibrary.MakeVector` (- _returnvalue_x 1.0) _returnvalue_y _returnvalue_z) true))

(fn `WalkForward`
  (bind (_returnvalue_x _returnvalue_y _returnvalue_z) (`KismetMathLibrary.BreakVector` (`self.K2_GetActorLocation`)))
  (`self.K2_SetActorLocation` (`KismetMathLibrary.MakeVector` (+ _returnvalue_x 1.0) _returnvalue_y _returnvalue_z) true))