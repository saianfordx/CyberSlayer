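; Paper2D robot enemy that patrols along X around its spawn point and shoots at the player when it spots them.
; Each Tick it checks life, then a sphere trace finds MyCharacter and a line trace confirms visibility, pausing patrol.
; While watching, it alternates spawning Bullets with a delayed idle.
; AnyDamage updates the life bar widget but passes zero damage; DetectPlayer and LookAt are unused.
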(event `self.ReceiveAnyDamage`
  (params (Damage :type "Float (single-precision)") (DamageType :type "DamageType Object Reference") (InstigatedBy :type "Controller Object Reference") (DamageCauser :type "Actor Object Reference"))
  (`self.SelfApplyDamage` 0.0))

(event `self.ReceiveBeginPlay`
  ;[1 1 1] Set Initial Variables
  (`self.SetInitialLocation`)
  (`self.SetMaxDistance`)
  (`self.SetMinDistance`)
  (`self.SetInitialLife`))

(event `self.ReceiveTick`
  (params (DeltaSeconds :type "Float (single-precision)"))
  (bind _isalive (`self.CheckActorLife`))
  (if _isalive
    ;[1 1 1] Look For Player In The Area
    (bind (_isplayerinthearea _character) (`self.CheckPlayerInTheArea`))
    (if _isplayerinthearea
      ;[1 1 1] If Player In The Area, Try To Find It
      (`self.RayCast` _character)
      (else
        (set `self.IsWatchingPlayer` false)))
    ;[1 1 1] Patrol / Walking Logic
    (`self.Patrol`)
    ;[1 1 1] Validate If Watching Player
    (if (`self.IsWatchingPlayer`)
      ;[1 1 1] Validate If Enemy Is Shooting
      (if (`self.isShooting`)
        ;[1 1 1] Set IDLE Animation
        (`PaperFlipbookComponent.SetFlipbook` (`self.PaperFlipbook`) "/Game/Migrations/2DSideScrollerBP/Semana_05/2DSideScrollerBP/Blueprints/Animations/Robot/Robot_Idle_FB.Robot_Idle_FB")
        ;[1 1 1] Next Shoot Delay
        (`KismetSystemLibrary.Delay` (`self.ShootingDelay`))
        ;[1 1 1] Stop Shooting Cicle
        (set `self.isShooting` false)
        (else
          ;[1 1 1] Start Shooting
          (`self.Shoot`)
          (set `self.isShooting` true))))))

(fn `AdjustPatrolDirection`
  (bind _returnvalue_x (`KismetMathLibrary.BreakVector` (`self.K2_GetActorLocation`)))
  (bind _returnvalue_x_2 (`KismetMathLibrary.BreakVector` (`self.K2_GetActorLocation`)))
  (if (>= _returnvalue_x_2 (`self.MaxDistance_X`))
    (set `self.Direction` -1.0)
    (elif (<= (`KismetMathLibrary.Abs` _returnvalue_x) (`KismetMathLibrary.Abs` (`self.MinDistance_X`)))
      (set `self.Direction` 1.0))))

(fn `CheckActorLife`
  (returns (IsAlive :type Boolean))
  (if (> (`self.Life`) 0.0)
    (return true)
    (else
      (`self.K2_DestroyActor`)
      (return false))))

(fn `CheckPlayerInTheArea`
  (returns (IsPlayerInTheArea :type Boolean) (Character :type "Actor Object Reference"))
  (bind _returnvalue (`self.K2_GetActorLocation`))
  (bind _outhits (`KismetSystemLibrary.SphereTraceMulti` _returnvalue _returnvalue 150.0 "TraceTypeQuery1"))
  (for _array_element _outhits
    (bind (_bblockinghit _binitialoverlap _time _distance _location _impactpoint _normal _impactnormal _physmat _hitactor) (`GameplayStatics.BreakHitResult` _array_element))
    (if (`KismetStringLibrary.Contains` (`KismetSystemLibrary.GetDisplayName` _hitactor) "MyCharacter")
      (bind _ascharacter (cast `Character` _hitactor))
      (set `self.IsPlayerInTheArea` true)
      (return true _ascharacter)))
  (set `self.IsPlayerInTheArea` false)
  (return false null))

(fn `DetectPlayer`
  (returns (Character :type "Actor Object Reference"))
  (bind _returnvalue (`self.K2_GetActorLocation`))
  (bind _outhit (`KismetSystemLibrary.LineTraceSingle` _returnvalue (+ _returnvalue (* (`KismetMathLibrary.GetForwardVector` (`self.K2_GetActorRotation`)) 100)) "TraceTypeQuery1"))
  (bind (_bblockinghit _binitialoverlap _time _distance _location _impactpoint _normal _impactnormal _physmat _hitactor) (`GameplayStatics.BreakHitResult` _outhit))
  (if (`KismetStringLibrary.Contains` (`KismetSystemLibrary.GetDisplayName` _hitactor) "MyCharacter")
    (set `self.IsWatchingPlayer` true)
    (bind _ascharacter (cast `Character` _hitactor))
    (return _ascharacter)
    (else
      (set `self.IsWatchingPlayer` false)
      (set `self.IsPlayerInTheArea` false))))

(fn `LookAt`
  (params (IsPlayerInTheArea :type Boolean))
  (if IsPlayerInTheArea
    (bind _returnvalue (`GameplayStatics.GetActorOfClass` "/Game/Migrations/2DSideScrollerBP/Semana_05/2DSideScrollerBP/Blueprints/MyCharacter.MyCharacter_C"))
    (`self.K2_SetActorRotation` (`self.K2_GetActorRotation` _returnvalue))))

(fn `Patrol`
  (if (not (`self.IsWatchingPlayer`))
    (`self.AdjustPatrolDirection`)
    (`self.RotateActor`)
    (`self.SetWalkingAnimation`)
    (if (>= (`self.Direction`) 0.0)
      (`self.WalkForward` 0.0)
      (else
        (`self.WalkBackward` 0.0)))))

(fn `RayCast`
  (params (PlayerInstance :type "Actor Object Reference"))
  (bind _outhit (`KismetSystemLibrary.LineTraceSingle` (`self.K2_GetActorLocation`) (`self.K2_GetActorLocation` PlayerInstance) "TraceTypeQuery1"))
  (if (`KismetStringLibrary.Contains` (`KismetSystemLibrary.GetDisplayName` (`.HitActor` (`GameplayStatics.BreakHitResult` _outhit))) "MyCharacter")
    (set `self.IsWatchingPlayer` true)
    (else
      (set `self.IsWatchingPlayer` false)
      (set `self.IsPlayerInTheArea` false))))

(fn `RotateActor`
  (bind _paperflipbook (`self.PaperFlipbook`))
  (if (>= (`self.Direction`) 0.0)
    (`SceneComponent.K2_SetRelativeRotation` :`self` _paperflipbook)
    (else
      (`SceneComponent.K2_SetRelativeRotation` _paperflipbook (struct :`Yaw` 180.0) false false))))

(fn `SelfApplyDamage`
  (params (Damage :type "Float (double-precision)"))
  (set `self.Life` (- (`self.Life`) Damage))
  (`self.UpdateLifeBar`))

(fn `SetInitialLife`
  (set `self.Life` (`self.MaxLife`)))

(fn `SetInitialLocation`
  (bind _returnvalue_x (`KismetMathLibrary.BreakVector` (`self.K2_GetActorLocation`)))
  (set `self.InitialLocation_X` _returnvalue_x))

(fn `SetMaxDistance`
  (set `self.MaxDistance_X` (+ (`self.PatrolRange`) (`self.InitialLocation_X`))))

(fn `SetMinDistance`
  (set `self.MinDistance_X` (- (`self.PatrolRange`) (`self.InitialLocation_X`))))

(fn `SetWalkingAnimation`
  (`PaperFlipbookComponent.SetFlipbook` (`self.PaperFlipbook`) "/Game/Logical_And_/Blueprints/Animations/Robot/Robot_Run_FB.Robot_Run_FB"))

(fn `Shoot`
  (`PaperFlipbookComponent.SetFlipbook` (`self.PaperFlipbook`) "/Game/Logical_And_/Blueprints/Animations/Robot/Robot_Shoot_FB.Robot_Shoot_FB")
  (`|SpawnActorFromClass` "/Game/Logical_And_/Blueprints/Actors/Bullet.Bullet_C" (`self.GetTransform`) "Undefined" "OverrideRootScale" null null)
  (set `self.isShooting` true))

(fn `UpdateLifeBar`
  (bind _asenemy_life_bar_wg (cast `/Game/Logical_And_/Blueprints/Widgets/Enemy_LifeBar_WG` (`WidgetComponent.GetUserWidgetObject` (`self.Widget`))))
  (`ProgressBar.SetPercent` (`/Game/Logical_And_/Blueprints/Widgets/Enemy_LifeBar_WG.ProgressBar_0` _asenemy_life_bar_wg) (/ (`self.Life`) (`self.MaxLife`))))

(fn `UserConstructionScript`)

(fn `WalkBackward`
  (params (DeltaTime :type "Float (double-precision)"))
  (bind (_returnvalue_x _returnvalue_y _returnvalue_z) (`KismetMathLibrary.BreakVector` (`self.K2_GetActorLocation`)))
  (`self.K2_SetActorLocation` (`KismetMathLibrary.MakeVector` (- _returnvalue_x 1.0) _returnvalue_y _returnvalue_z) true))

(fn `WalkForward`
  (params (DeltaTime :type "Float (double-precision)"))
  (bind (_returnvalue_x _returnvalue_y _returnvalue_z) (`KismetMathLibrary.BreakVector` (`self.K2_GetActorLocation`)))
  (`self.K2_SetActorLocation` (`KismetMathLibrary.MakeVector` (+ (* (`GameplayStatics.GetWorldDeltaSeconds`) (`self.Speed`)) _returnvalue_x) _returnvalue_y _returnvalue_z) true))