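; DropTrapTrigger is a trigger actor that starts a falling trap when the player comes near it.
; Every tick it sphere-traces a small radius at its location and identifies the player by "MyCharacter" in the hit actor's display name.
; A hit clears IsActive, which stops further detection only when IsOneTimeDamage is set, and calls StartFalling on whichever FallingTrap GetActorOfClass returns, with no explicit link.
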(event `self.ReceiveTick`
  (params (DeltaSeconds :type "Float (single-precision)"))
  (if (`self.isOneTimeDamage`)
    (if (`self.isActive`)
      (`self.detectPlayer`))
    (else
      (`self.detectPlayer`))))

(fn `activateFalling`
  (bind _returnvalue (`GameplayStatics.GetActorOfClass` "/Game/Logical_And_/Blueprints/Actors/FallingTrap.FallingTrap_C"))
  (`/Game/Logical_And_/Blueprints/Actors/FallingTrap.startFalling` _returnvalue))

(fn `detectPlayer`
  (returns (trapActive :type Boolean))
  (bind _returnvalue (`self.K2_GetActorLocation`))
  (bind _outhits (`KismetSystemLibrary.SphereTraceMulti` _returnvalue _returnvalue 30.0 "TraceTypeQuery1"))
  (for _array_element _outhits
    (if (`KismetStringLibrary.Contains` (`KismetSystemLibrary.GetDisplayName` (`.HitActor` (`GameplayStatics.BreakHitResult` _array_element))) "MyCharacter")
      (`GameplayStatics.GetActorOfClass` "/Game/Logical_And_/Blueprints/Actors/Player/MyCharacter.MyCharacter_C")
      (set `self.isActive` false)
      (`self.activateFalling`)
      (return true))))

(fn `UserConstructionScript`)