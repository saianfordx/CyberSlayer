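; Three-phase Paper2D boss that turns from evil wizard to fire knight to demon as Life drops, then shows the game-finished menu on death.
; Tick sets the phase by Life thresholds and runs transforms, flipbook swaps and arena fire spawns, pacing attacks with Delays.
; The wizard spawns projectile patterns, the knight dashes or drops gapped volleys, and the demon patrols, casts and cleaves.
; Melee hits use sphere traces matched on the player's display name.
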(event `self.ReceiveBeginPlay`)

(event `self.ReceiveTick`
  (params (DeltaSeconds :type "Float (single-precision)"))
  (bind (_returnvalue_x _returnvalue_y _returnvalue_z) (`KismetMathLibrary.BreakVector` (`self.K2_GetActorLocation`)))
  (bind (_returnvalue_x_2 _returnvalue_y_2 _returnvalue_z_2) (`KismetMathLibrary.BreakVector` (`self.K2_GetActorLocation`)))
  (if (> (`self.Life`) 0.0)
    (`self.Mode_Index_Manager`)
    (if (and (`self.isElemental`) (== (`self.didElementalTransform`) false))
      (set `self.didElementalTransform` true)
      (set `self.Current_Mode` 2)
      (`self.Spawn_Lava_Floor`)
      (`self.Spawn_Torch_01`)
      (`self.Elemental_Transform`)
      (`KismetSystemLibrary.Delay` 0.8)
      (`self.Set_Eelemental_FireKnight_Idle`)
      (else
        (switch `int` (`self.Current_Mode`)
          (:`1`
            (`KismetSystemLibrary.Delay` 4.0)
            (bind _index (`self.Atack_Index_Manager_Generator` 1 4))
            (`self.Atack_Index_Manager_Executer` _index)
            (`KismetSystemLibrary.Delay` 1.0)
            (`self.Set_Idle_FB`))
          (:`2`
            (if (`self.isAtacking`)
              (switch `int` (`self.Current_Atack`)
                (:`1`
                  (`self.Elemental_FireKnight_Atack_Manager` (`self.Current_Atack`)))
                (:`2`
                  (`self.Sawn_Fire_FX`)
                  (`self.Elemental_FireKnight_Atack_Manager` (`self.Current_Atack`))
                  (`KismetSystemLibrary.Delay` 0.5)
                  (`self.K2_SetActorLocation` (`KismetMathLibrary.MakeVector` 220.0 _returnvalue_y_2 _returnvalue_z_2) true)
                  (`KismetSystemLibrary.Delay` 0.5)
                  (`self.Set_Eelemental_FireKnight_Idle`)
                  (`self.K2_SetActorLocation` (`KismetMathLibrary.MakeVector` 30.0 _returnvalue_y _returnvalue_z) true)
                  (set `self.isAtacking` false))
                (:`3`
                  (`self.Elemental_FireKnight_Atack_Manager` (`self.Current_Atack`))))
              (else
                (`KismetSystemLibrary.Delay` 2.0)
                (bind _index_2 (`self.Atack_Index_Manager_Generator` 1 3))
                (`self.Elemental_FireKnight_Atack_Manager` _index_2))))
          (:`3`
            (if (`self.didDemonTransform`)
              (if (not (`self.isTranforming`))
                (`self.Demon Get Player Direction`)
                (bind _player_detected (`self.Demon_Detect_Player`))
                (if _player_detected
                  (`self.Demon_Slash`)
                  (elif (`self.isDemonAtacking`)
                    (switch `int` (`self.Current_Demon_Atack`)
                      (:`1`
                        (`self.Demon_Atack_Manager` 0)
                        (`KismetSystemLibrary.Delay` 2.0)
                        (set `self.isDemonAtacking` false)))
                    (else
                      (`self.Demon_Patrol`)
                      (`KismetSystemLibrary.Delay` 2.0)
                      (bind _index_3 (`self.Atack_Index_Manager_Generator` 1 1))
                      (`self.Demon_Atack_Manager` _index_3)))))
              (else
                (set `self.isTranforming` true)
                (set `self.isAtacking` false)
                (`KismetSystemLibrary.Delay` 1.0)
                (set `self.isDemon` true)
                (`self.Set_Demon_Transform`)
                (`KismetSystemLibrary.Delay` 6.0)
                (`GameplayStatics.SpawnSound2D` "/Game/2DSideScrollerBP/Sound/Effects/demonVoice_Cue.demonVoice_Cue" 1.0 1.0 0.0 null)
                (set `self.didDemonTransform` true)
                (`self.Set_Demon_Idle`)
                (set `self.isTranforming` false)
                (`self.Spawn_Fire_Background`)))))))
    (else
      (`self.Set_Demon_Death`)
      (`KismetSystemLibrary.Delay` 4.0)
      (`self.Finish_Game`)
      (`self.K2_DestroyActor`))))

(fn `Atack_01`
  (for _index (range 1 8)
    (if (<= _index 7)
      (`|SpawnActorFromClass` "/Game/Logical_And_/Blueprints/Actors/Boss/Boss_Base_Atack_BP.Boss_Base_Atack_BP_C" (`KismetMathLibrary.MakeTransform` (`KismetMathLibrary.MakeVector` (`KismetMathLibrary.Conv_IntToDouble` (`self.spawn_counter_atack_01`)))) "Undefined" "OverrideRootScale" null null)
      (set `self.spawn_counter_atack_01` (+ (`self.spawn_counter_atack_01`) 70))))
  (set `self.spawn_counter_atack_01` 0))

(fn `Atack_02`
  (bind (_returnvalue_x _returnvalue_y) (`KismetMathLibrary.BreakVector` (`self.K2_GetActorLocation`)))
  (for _index (range 1 8)
    (if (<= _index 7)
      (bind _returnvalue (`|SpawnActorFromClass` "/Game/Logical_And_/Blueprints/Actors/Boss/Boss_Base_Atack_Horizontal_BP_.Boss_Base_Atack_Horizontal_BP__C" (`KismetMathLibrary.MakeTransform` (`KismetMathLibrary.MakeVector` _returnvalue_x _returnvalue_y (`KismetMathLibrary.Conv_IntToDouble` (`self.spawn_counter_atack_02`)))) "Undefined" "OverrideRootScale" null null))
      (set `self.spawn_counter_atack_02` (+ (`self.spawn_counter_atack_02`) 70))
      (bind _asboss_base_atack_horizontal_bp_ (cast `/Game/Logical_And_/Blueprints/Actors/Boss/Boss_Base_Atack_Horizontal_BP_` _returnvalue))
      (set `/Game/Logical_And_/Blueprints/Actors/Boss/Boss_Base_Atack_Horizontal_BP_.isForward` (`self.isForward`) _asboss_base_atack_horizontal_bp_)))
  (set `self.spawn_counter_atack_02` -280))

(fn `Atack_03`
  (bind (_returnvalue_x _returnvalue_y _returnvalue_z) (`KismetMathLibrary.BreakVector` (`self.K2_GetActorLocation`)))
  (bind (_returnvalue_x_2 _returnvalue_y_2 _returnvalue_z_2) (`KismetMathLibrary.BreakVector` (`self.K2_GetActorLocation`)))
  (bind (_returnvalue_x_3 _returnvalue_y_3 _returnvalue_z_3) (`KismetMathLibrary.BreakVector` (`self.K2_GetActorLocation`)))
  (if (> _returnvalue_x 40.0)
    (`self.K2_SetActorLocation` (`KismetMathLibrary.MakeVector` 40.0 _returnvalue_y _returnvalue_z))
    (`SceneComponent.K2_SetRelativeRotation` :`self` (`self.PaperFlipbook`))
    (for _index (range 1 2)
      (if (<= _index 7)
        (bind _returnvalue (`|SpawnActorFromClass` "/Game/Logical_And_/Blueprints/Actors/Boss/Boss_Base_Atack_Horizontal_BP_.Boss_Base_Atack_Horizontal_BP__C" (`KismetMathLibrary.MakeTransform` (`KismetMathLibrary.MakeVector` _returnvalue_x_2 _returnvalue_y_2 _returnvalue_z_2)) "Undefined" "OverrideRootScale" null null))
        (bind _asboss_base_atack_horizontal_bp_ (cast `/Game/Logical_And_/Blueprints/Actors/Boss/Boss_Base_Atack_Horizontal_BP_` _returnvalue))
        (bind _output_get (set `/Game/Logical_And_/Blueprints/Actors/Boss/Boss_Base_Atack_Horizontal_BP_.isForward` true _asboss_base_atack_horizontal_bp_))
        (set `self.isForward` _output_get)))
    (else
      (`self.K2_SetActorLocation` (`KismetMathLibrary.MakeVector` 390.0 _returnvalue_y _returnvalue_z))
      (`SceneComponent.K2_SetRelativeRotation` (`self.PaperFlipbook`) (struct :`Yaw` 180.0) false false)
      (for _index_2 (range 1 2)
        (if (<= _index_2 7)
          (bind _returnvalue_2 (`|SpawnActorFromClass` "/Game/Logical_And_/Blueprints/Actors/Boss/Boss_Base_Atack_Horizontal_BP_.Boss_Base_Atack_Horizontal_BP__C" (`KismetMathLibrary.MakeTransform` (`KismetMathLibrary.MakeVector` _returnvalue_x_3 _returnvalue_y_3 _returnvalue_z_3)) "Undefined" "OverrideRootScale" null null))
          (bind _asboss_base_atack_horizontal_bp__2 (cast `/Game/Logical_And_/Blueprints/Actors/Boss/Boss_Base_Atack_Horizontal_BP_` _returnvalue_2))
          (bind _output_get_2 (set `/Game/Logical_And_/Blueprints/Actors/Boss/Boss_Base_Atack_Horizontal_BP_.isForward` false _asboss_base_atack_horizontal_bp__2))
          (set `self.isForward` _output_get_2))))))

(fn `Atack_04`
  (for _index (range 1 20)
    (if (<= _index 19)
      (`|SpawnActorFromClass` "/Game/Logical_And_/Blueprints/Actors/Boss/Boss_Fire_BP.Boss_Fire_BP_C" (`KismetMathLibrary.MakeTransform` (`KismetMathLibrary.MakeVector` (`KismetMathLibrary.Conv_IntToDouble` (`self.spawn_counter_atack_03`)) 0.0 -250.0)) "Undefined" "OverrideRootScale" null null)
      (set `self.spawn_counter_atack_03` (+ (`self.spawn_counter_atack_03`) 25))))
  (set `self.spawn_counter_atack_03` 0))

(fn `Atack_Index_Manager_Executer`
  (params (Index :type Integer))
  (if (== (`self.Current_Mode`) 1)
    (if (> (`self.Life`) 0.0)
      (`self.Set_Atack_01_FB`)
      (switch `int` Index
        (:`1`
          (`self.Atack_01`))
        (:`2`
          (`self.Atack_02`))
        (:`3`
          (`self.Atack_03`))
        (:`4`
          (`self.Atack_04`))))))

(fn `Atack_Index_Manager_Generator`
  (params (Min :type Integer) (Max :type Integer))
  (returns (Index :type Integer))
  (return (`KismetMathLibrary.RandomIntegerInRange` Min Max)))

(fn `Atack_Transform_Manager`
  (switch `int` (`self.Current_Mode`)
    (:`0`
      (`self.Atack_Index_Manager_Executer` 0))
    (:`1`
      (`self.Atack_Transform_Manager`))))

(fn `Demon Get Player Direction`
  (bind _returnvalue_x (`KismetMathLibrary.BreakVector` (`self.K2_GetActorLocation`)))
  (bind _returnvalue (`GameplayStatics.GetActorOfClass` "/Game/Logical_And_/Blueprints/Actors/Player/MyCharacter.MyCharacter_C"))
  (bind _returnvalue_x_2 (`KismetMathLibrary.BreakVector` (`self.K2_GetActorLocation` _returnvalue)))
  (if (>= _returnvalue_x_2 _returnvalue_x)
    (set `self.PlayerDirection` 1.0)
    (`SceneComponent.K2_SetRelativeRotation` (`self.PaperFlipbook`) (struct :`Yaw` 180.0) false false)
    (else
      (set `self.PlayerDirection` -1.0)
      (`SceneComponent.K2_SetRelativeRotation` :`self` (`self.PaperFlipbook`)))))

(fn `Demon_Ad`)

(fn `Demon_Atack_01`
  (bind (_returnvalue_x _returnvalue_y _returnvalue_z) (`KismetMathLibrary.BreakVector` (`self.K2_GetActorLocation`)))
  (bind (_returnvalue_x_2 _returnvalue_y_2 _returnvalue_z_2) (`KismetMathLibrary.BreakVector` (`self.K2_GetActorLocation`)))
  (if (not (`self.isDemonAtacking`))
    (`PaperFlipbookComponent.SetFlipbook` (`self.PaperFlipbook`) "/Game/Logical_And_/Blueprints/Animations/Demon/Fire_Breat/Demon_Fire_Breat_FB.Demon_Fire_Breat_FB")
    (if (> (`self.PlayerDirection`) 0.0)
      (`|SpawnActorFromClass` "/Game/Logical_And_/Blueprints/Actors/Boss/Fire_Breath_BP.Fire_Breath_BP_C" (`KismetMathLibrary.MakeTransform` (`KismetMathLibrary.MakeVector` (+ _returnvalue_x 80.0) _returnvalue_y (+ _returnvalue_z 40.0))) "Undefined" "OverrideRootScale" null null)
      (else
        (`|SpawnActorFromClass` "/Game/Logical_And_/Blueprints/Actors/Boss/Fire_Breath_BP.Fire_Breath_BP_C" (`KismetMathLibrary.MakeTransform` (`KismetMathLibrary.MakeVector` (- _returnvalue_x_2 80.0) _returnvalue_y_2 (+ _returnvalue_z_2 40.0))) "Undefined" "OverrideRootScale" null null)))
    (set `self.isDemonAtacking` true)))

(fn `Demon_Atack_Manager`
  (params (Index :type Integer))
  (switch `int` Index
    (:`1`
      (set `self.Current_Demon_Atack` 1)
      (`self.Set_Demon_Cast`)
      (`self.Elemental_FireKnight_Atack_03`)
      (set `self.isDemonAtacking` true))))

(fn `Demon_Damage_Detection`
  (params (Range :type Integer))
  (bind _returnvalue (`self.K2_GetActorLocation`))
  (bind _outhits (`KismetSystemLibrary.SphereTraceMulti` _returnvalue _returnvalue (`KismetMathLibrary.Conv_IntToDouble` Range) "TraceTypeQuery1"))
  (for _array_element _outhits
    (if (`KismetStringLibrary.Contains` (`KismetSystemLibrary.GetDisplayName` (`.HitActor` (`GameplayStatics.BreakHitResult` _array_element))) "MyCharacter")
      (bind _returnvalue_2 (`GameplayStatics.GetActorOfClass` "/Game/Logical_And_/Blueprints/Actors/Player/MyCharacter.MyCharacter_C"))
      (`GameplayStatics.ApplyDamage` _returnvalue_2 (`self.Demon_Damage`))
      (bind _returnvalue_3 (`|SpawnActorFromClass` "/Game/Logical_And_/Blueprints/Animations/Explotions/Explotion_01/Explotion_01_BP.Explotion_01_BP_C" (`self.GetTransform`) "Undefined" "OverrideRootScale" null null))
      (`self.K2_DestroyActor` _returnvalue_3)
      (set `self.didDemonHit` true))))

(fn `Demon_Detect_Player`
  (returns (Player_Detected :type Boolean))
  (bind _returnvalue (`self.K2_GetActorLocation`))
  (bind _outhits (`KismetSystemLibrary.SphereTraceMulti` _returnvalue _returnvalue 100.0 "TraceTypeQuery1"))
  (for _array_element _outhits
    (if (`KismetStringLibrary.Contains` (`KismetSystemLibrary.GetDisplayName` (`.HitActor` (`GameplayStatics.BreakHitResult` _array_element))) "MyCharacter")
      (return true)))
  (return false))

(fn `Demon_Patrol`
  (bind _returnvalue_x (`KismetMathLibrary.BreakVector` (`self.K2_GetActorLocation`)))
  (bind _returnvalue_x_2 (`KismetMathLibrary.BreakVector` (`self.K2_GetActorLocation`)))
  (bind (_returnvalue_x_3 _returnvalue_y _returnvalue_z) (`KismetMathLibrary.BreakVector` (`self.K2_GetActorLocation`)))
  (bind (_returnvalue_x_4 _returnvalue_y_2 _returnvalue_z_2) (`KismetMathLibrary.BreakVector` (`self.K2_GetActorLocation`)))
  (if (>= _returnvalue_x_2 (`self.Max_Distance_X`))
    (set `self.PlayerDirection` -1.0)
    (`self.K2_SetActorLocation` (`KismetMathLibrary.MakeVector` (- _returnvalue_x_3 (* (`self.demon_speed_tempo`) (`GameplayStatics.GetWorldDeltaSeconds`))) _returnvalue_y _returnvalue_z) :!label _label)
    (else
      (if (<= (`KismetMathLibrary.Abs` _returnvalue_x) (`KismetMathLibrary.Abs` (`self.Min_Distance_X`)))
        (set `self.PlayerDirection` 1.0)
        (elif (> (`self.PlayerDirection`) 0.0)
          _
          (else
            (goto _label))))
      (`self.K2_SetActorLocation` (`KismetMathLibrary.MakeVector` (+ (* (`self.demon_speed_tempo`) (`GameplayStatics.GetWorldDeltaSeconds`)) _returnvalue_x_4) _returnvalue_y_2 _returnvalue_z_2))))
  (`self.Set_Demon_Walk`))

(fn `Demon_Slash`
  (if (not (`self.isDemonAtacking`))
    (`PaperFlipbookComponent.SetFlipbook` (`self.PaperFlipbook`) "/Game/Logical_And_/Blueprints/Animations/Demon/Cleave/Demon_Cleave_FB.Demon_Cleave_FB")
    (`self.Demon_Damage_Detection` 80)))

(fn `Detect_Player`
  (params (Range :type "Float (double-precision)"))
  (bind _returnvalue (`self.K2_GetActorLocation`))
  (bind _outhits (`KismetSystemLibrary.SphereTraceMulti` _returnvalue _returnvalue Range "TraceTypeQuery1"))
  (for _array_element _outhits
    (if (`KismetStringLibrary.Contains` (`KismetSystemLibrary.GetDisplayName` (`.HitActor` (`GameplayStatics.BreakHitResult` _array_element))) "MyCharacter")
      (bind _returnvalue_2 (`GameplayStatics.GetActorOfClass` "/Game/Logical_And_/Blueprints/Actors/Player/MyCharacter.MyCharacter_C"))
      (`GameplayStatics.ApplyDamage` _returnvalue_2 (`self.Damage`))
      (bind _returnvalue_3 (`|SpawnActorFromClass` "/Game/Logical_And_/Blueprints/Animations/Explotions/Explotion_01/Explotion_01_BP.Explotion_01_BP_C" (`self.GetTransform`) "Undefined" "OverrideRootScale" null null))
      (`self.K2_DestroyActor` _returnvalue_3))))

(fn `Elemenental_FireKnight_Atack_02_Movement`)

(fn `Elemental_FireKnight_Atack_01`
  (if (!= (`self.PaperFlipbook`) "/Game/Logical_And_/Blueprints/Animations/Fire_Knight/Atack_03/Elemental_Knight_Atack_03_FB.Elemental_Knight_Atack_03_FB")
    (`PaperFlipbookComponent.SetFlipbook` (`self.PaperFlipbook`) "/Game/2DSideScrollerBP/Blueprints/Animations/Fire_Knight/Atack_03/Fire_Knight_Atack_03_FB.Fire_Knight_Atack_03_FB"))
  (`self.Set_Direction`)
  (set `self.isAtacking` true)
  (`self.Detect_Player` 30.0)
  (`self.Move2`))

(fn `Elemental_FireKnight_Atack_02`
  (if (!= (`self.PaperFlipbook`) "/Game/2DSideScrollerBP/Blueprints/Animations/Fire_Knight/Atack_04/Fire_Knight_Atack_04_FB.Fire_Knight_Atack_04_FB")
    (`PaperFlipbookComponent.SetFlipbook` (`self.PaperFlipbook`) "/Game/2DSideScrollerBP/Blueprints/Animations/Fire_Knight/Atack_04/Fire_Knight_Atack_04_FB.Fire_Knight_Atack_04_FB"))
  (`self.Set_Direction`)
  (set `self.isAtacking` true)
  (`self.Detect_Player` 50.0))

(fn `Elemental_FireKnight_Atack_03`
  (bind _returnvalue (`KismetMathLibrary.RandomIntegerInRange` 1 15))
  (set `self.isAtacking` true)
  (while (<= (`KismetArrayLibrary.Array_Length` (`self.Randoms`)) 5)
    (if (not (> (`KismetArrayLibrary.Array_Find` (`self.Randoms`) _returnvalue) 0))
      (`KismetArrayLibrary.Array_Add` (`self.Randoms`) _returnvalue)))
  (for _ (`self.Randoms`)
    (for _index (range 1 16)
      (if (not (> (`KismetArrayLibrary.Array_Find` (`self.Randoms`) _index) 0))
        (`|SpawnActorFromClass` "/Game/Logical_And_/Blueprints/Actors/Boss/Boss_Base_Atack_Eelemental_BP_.Boss_Base_Atack_Eelemental_BP__C" (`KismetMathLibrary.MakeTransform` (`KismetMathLibrary.MakeVector` (`KismetMathLibrary.Conv_IntToDouble` (`self.spawn_counter_atack_FK_01`)))) "Undefined" "OverrideRootScale" null null))
      (set `self.spawn_counter_atack_FK_01` (+ (`self.spawn_counter_atack_FK_01`) 30))
      (set `self.isAtacking` false))
    (set `self.spawn_counter_atack_FK_01` 0)
    (`KismetArrayLibrary.Array_Clear` (`self.Randoms`))))

(fn `Elemental_FireKnight_Atack_Manager`
  (params (index :type Integer))
  (switch `int` index
    (:`1`
      (set `self.Current_Atack` 1)
      (`self.Elemental_FireKnight_Atack_01`))
    (:`2`
      (set `self.Current_Atack` 2)
      (`self.Elemental_FireKnight_Atack_02`))
    (:`3`
      (set `self.Current_Atack` 3)
      (`self.Elemental_FireKnight_Atack_03`))))

(fn `Elemental_Transform`
  (bind _paperflipbook (`self.PaperFlipbook`))
  (bind _returnvalue (`SceneComponent.GetRelativeTransform` _paperflipbook))
  (`SceneComponent.K2_SetRelativeLocation` _paperflipbook (`KismetMathLibrary.MakeVector` (.x (.location _returnvalue)) (.y (.location _returnvalue)) 45.0) false false)
  (`PaperFlipbookComponent.SetFlipbook` (`self.PaperFlipbook`) "/Game/2DSideScrollerBP/Blueprints/Animations/Fire_Knight/Transform/Fire_Knight_Transform_FB.Fire_Knight_Transform_FB"))

(fn `Finish_Game`
  (bind _returnvalue (`|CreateWidget` "/Game/2DSideScrollerBP/Blueprints/Menus/InGame_Menu/GameFinished_Menu.GameFinished_Menu_C"))
  (`UserWidget.AddToViewport` _returnvalue 0))

(fn `Get_Current_Life`
  (returns (CurrentLife :type "Float (double-precision)"))
  (return (`self.Life`)))

(fn `Mode_Index_Manager`
  (if (and (== (`self.isElemental`) true) (<= (`self.Life`) 150.0))
    (set `self.Current_Mode` 3)
    (set `self.isDemon` true)
    (elif (and (<= (`self.Life`) 250.0) (== (`self.isElemental`) false))
      (set `self.Current_Mode` 2)
      (set `self.isElemental` true))))

(fn `Move2`
  (bind _returnvalue_x (`KismetMathLibrary.BreakVector` (`self.K2_GetActorLocation`)))
  (bind (_returnvalue_x_2 _returnvalue_y _returnvalue_z) (`KismetMathLibrary.BreakVector` (`self.K2_GetActorLocation`)))
  (bind (_returnvalue_x_3 _returnvalue_y_2 _returnvalue_z_2) (`KismetMathLibrary.BreakVector` (`self.K2_GetActorLocation`)))
  (bind _returnvalue_x_4 (`KismetMathLibrary.BreakVector` (`self.K2_GetActorLocation`)))
  (if (`self.isForward`)
    (if (>= (`KismetMathLibrary.Abs` _returnvalue_x_4) (`KismetMathLibrary.Abs` (`self.Max_Distance_X`)))
      (set `self.Current_Atack` 0)
      (set `self.isAtacking` false)
      (`self.Set_Eelemental_FireKnight_Idle` :!label _label)
      (`self.Set_Direction`)
      (else
        (`self.K2_SetActorLocation` (`KismetMathLibrary.MakeVector` (+ (* (`self.Speed_Tempo`) (`GameplayStatics.GetWorldDeltaSeconds`)) _returnvalue_x_3) _returnvalue_y_2 _returnvalue_z_2) true)))
    (elif (<= (`KismetMathLibrary.Abs` _returnvalue_x) (`KismetMathLibrary.Abs` (`self.Min_Distance_X`)))
      (set `self.Current_Atack` 0)
      (set `self.isAtacking` false)
      (goto _label)
      (else
        (`self.K2_SetActorLocation` (`KismetMathLibrary.MakeVector` (- _returnvalue_x_2 (* (`self.Speed_Tempo`) (`GameplayStatics.GetWorldDeltaSeconds`))) _returnvalue_y _returnvalue_z) true)))))

(fn `Remove_Fire_Background`
  (bind _outactors (`GameplayStatics.GetAllActorsOfClass` "/Game/Logical_And_/Blueprints/Actors/Boss/Fire_Background_BP.Fire_Background_BP_C"))
  (for _array_element _outactors
    (bind _asfire_background_bp (cast `/Game/Logical_And_/Blueprints/Actors/Boss/Fire_Background_BP` _array_element))
    (`self.K2_DestroyActor` _asfire_background_bp)))

(fn `Sawn_Fire_FX`
  (bind (_returnvalue_x _returnvalue_y _returnvalue_z) (`KismetMathLibrary.BreakVector` (`self.K2_GetActorLocation`)))
  (`|SpawnActorFromClass` "/Game/Logical_And_/Blueprints/Actors/Boss/Fire_FX_01_BP.Fire_FX_01_BP_C" (`KismetMathLibrary.MakeTransform` (`KismetMathLibrary.MakeVector` 250.0 _returnvalue_y _returnvalue_z)) "Undefined" "OverrideRootScale" null null))

(fn `Self_Apply_Damage`
  (params (Damage :type "Float (double-precision)"))
  (if (not (`self.isTranforming`))
    (set `self.Life` (- (`self.Life`) Damage))
    (`self.Set_Take_Hit_FB`)))

(fn `Set_Atack_01_FB`
  (`PaperFlipbookComponent.SetFlipbook` (`self.PaperFlipbook`) "/Game/Logical_And_/Blueprints/Animations/Evil_Wizard/Atack_01/Evil_WizarD_Atack_01_FB.Evil_WizarD_Atack_01_FB"))

(fn `Set_Demon_Cast`
  (`PaperFlipbookComponent.SetFlipbook` (`self.PaperFlipbook`) "/Game/Logical_And_/Blueprints/Animations/Demon/Cast_Spell/Demon_Cast_Spell_FB.Demon_Cast_Spell_FB"))

(fn `Set_Demon_Death`
  (`PaperFlipbookComponent.SetFlipbook` (`self.PaperFlipbook`) "/Game/Logical_And_/Blueprints/Animations/Demon/Death/Demon_Death_FB.Demon_Death_FB"))

(fn `Set_Demon_Idle`
  (`PaperFlipbookComponent.SetFlipbook` (`self.PaperFlipbook`) "/Game/Logical_And_/Blueprints/Animations/Demon/Idle/Demon_Idle_FB.Demon_Idle_FB"))

(fn `Set_Demon_Transform`
  (bind _paperflipbook (`self.PaperFlipbook`))
  (bind _returnvalue (`SceneComponent.GetRelativeTransform` _paperflipbook))
  (`SceneComponent.K2_SetRelativeLocation` _paperflipbook (`KismetMathLibrary.MakeVector` (.x (.location _returnvalue)) (.y (.location _returnvalue)) 53.0) false false)
  (`PaperFlipbookComponent.SetFlipbook` (`self.PaperFlipbook`) "/Game/Logical_And_/Blueprints/Animations/Demon/Transform/Demon_Transform_FB.Demon_Transform_FB"))

(fn `Set_Demon_Walk`
  (`PaperFlipbookComponent.SetFlipbook` (`self.PaperFlipbook`) "/Game/Logical_And_/Blueprints/Animations/Demon/Walk/Demon_Walk_FB.Demon_Walk_FB"))

(fn `Set_Direction`
  (returns (IsForwaredReturn :type Boolean))
  (bind _returnvalue_x (`KismetMathLibrary.BreakVector` (`self.K2_GetActorLocation`)))
  (bind _returnvalue_x_2 (`KismetMathLibrary.BreakVector` (`self.K2_GetActorLocation`)))
  (if (`self.isAtacking`)
    _
    (elif (>= _returnvalue_x_2 (`self.Max_Distance_X`))
      (set `self.isForward` false)
      (`SceneComponent.K2_SetRelativeRotation` (`self.PaperFlipbook`) (struct :`Yaw` 180.0) false false)
      (return false)
      (elif (<= (`KismetMathLibrary.Abs` _returnvalue_x) (`KismetMathLibrary.Abs` (`self.Min_Distance_X`)))
        (set `self.isForward` true)
        (`SceneComponent.K2_SetRelativeRotation` :`self` (`self.PaperFlipbook`))
        (return true)))))

(fn `Set_Eelemental_FireKnight_Idle`
  (`PaperFlipbookComponent.SetFlipbook` (`self.PaperFlipbook`) "/Game/2DSideScrollerBP/Blueprints/Animations/Fire_Knight/Idle/Fire_Knight_Idle_FB.Fire_Knight_Idle_FB"))

(fn `Set_Idle_FB`
  (if (== (`self.Current_Mode`) 1)
    (`PaperFlipbookComponent.SetFlipbook` (`self.PaperFlipbook`) "/Game/Logical_And_/Blueprints/Animations/Evil_Wizard/Idle/Evil_Wizard_Idle_FB.Evil_Wizard_Idle_FB")))

(fn `Set_Take_Hit_FB`
  (if (not (`self.isElemental`))
    (`PaperFlipbookComponent.SetFlipbook` (`self.PaperFlipbook`) "/Game/Logical_And_/Blueprints/Animations/Evil_Wizard/Take_Hit/Evil_Wizard_Take_Hit_FB.Evil_Wizard_Take_Hit_FB")))

(fn `Spawn_Fire_Background`
  (if (not (`self.isFireSpawned`))
    (for _ (range 1 10)
      (`|SpawnActorFromClass` "/Game/Logical_And_/Blueprints/Actors/Boss/Fire_Background_BP.Fire_Background_BP_C" (`KismetMathLibrary.MakeTransform` (`KismetMathLibrary.MakeVector` (`self.spawn_fire_background_counter`) -10.0 -320.0)) "Undefined" "OverrideRootScale" null null)
      (set `self.spawn_fire_background_counter` (+ (`self.spawn_fire_background_counter`) 50.0))
      (set `self.isFireSpawned` true))
    (set `self.spawn_fire_background_counter` 18.0)))

(fn `Spawn_Lava_Floor`
  (for _ (range 11)
    (`|SpawnActorFromClass` "/Game/Logical_And_/Blueprints/Actors/Boss/Lava_Floor.Lava_Floor_C" (`KismetMathLibrary.MakeTransform` (`KismetMathLibrary.MakeVector` (`self.spawn_lava_floor_counter`) 5.0 -340.0)) "Undefined" "OverrideRootScale" null null)
    (set `self.spawn_lava_floor_counter` (+ (`self.spawn_lava_floor_counter`) 40.0)))
  (set `self.spawn_lava_floor_counter` 0.0))

(fn `Spawn_Torch_01`
  (`|SpawnActorFromClass` "/Game/Logical_And_/Blueprints/Actors/Boss/Torch_01_BP.Torch_01_BP_C" (`KismetMathLibrary.MakeTransform` (150.0 -5.0 -170.0)) "Undefined" "OverrideRootScale" null null)
  (`|SpawnActorFromClass` "/Game/Logical_And_/Blueprints/Actors/Boss/Torch_01_BP.Torch_01_BP_C" (`KismetMathLibrary.MakeTransform` (295.0 -5.0 -170.0)) "Undefined" "OverrideRootScale" null null))

(fn `UserConstructionScript`)