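; Boss fire breath projectile that moves straight down each Tick at a set Speed and damages the player.
; Until it hits, a small sphere trace looks for actors named like MyCharacter, applies damage, spawns an explosion actor and immediately calls DestroyActor on it.
; After a hit, detection stops and the projectile destroys itself only once below a fixed height, so misses are never cleaned up here.
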(event `self.ReceiveTick`
  (params (DeltaSeconds :type "Float (single-precision)"))
  (`self.Move`)
  (if (`self.hit`)
    (`self.Destroy_Actor`)
    (else
      (`self.Detect_Player`))))

(fn `Destroy_Actor`
  (bind (_returnvalue_x _returnvalue_y _returnvalue_z) (`KismetMathLibrary.BreakVector` (`self.K2_GetActorLocation`)))
  (if (< _returnvalue_z 300.0)
    (`self.K2_DestroyActor`)))

(fn `Detect_Player`
  (locals (Did_Hit :type Boolean))
  (bind _returnvalue (`self.K2_GetActorLocation`))
  (bind _outhits (`KismetSystemLibrary.SphereTraceMulti` :`Start` _returnvalue :`End` _returnvalue :`Radius` 20.0 :`TraceChannel` "TraceTypeQuery1" :`DrawDebugType` "ForOneFrame"))
  (for _array_element _outhits
    (if (`KismetStringLibrary.Contains` (`KismetSystemLibrary.GetDisplayName` (`.HitActor` (`GameplayStatics.BreakHitResult` _array_element))) "MyCharacter")
      (bind _returnvalue_2 (`GameplayStatics.GetActorOfClass` "/Game/Logical_And_/Blueprints/Actors/Player/MyCharacter.MyCharacter_C"))
      (`GameplayStatics.ApplyDamage` _returnvalue_2 (`self.Damage`))
      (bind _returnvalue_3 (`|SpawnActorFromClass` "/Game/Logical_And_/Blueprints/Animations/Explotions/Explotion_01/Explotion_01_BP.Explotion_01_BP_C" (`self.GetTransform`) "Undefined" "OverrideRootScale" null null))
      (`self.K2_DestroyActor` _returnvalue_3)
      (set `self.hit` true))))

(fn `Move`
  (bind (_returnvalue_x _returnvalue_y _returnvalue_z) (`KismetMathLibrary.BreakVector` (`self.K2_GetActorLocation`)))
  (`self.K2_SetActorLocation` (`KismetMathLibrary.MakeVector` _returnvalue_x _returnvalue_y (- _returnvalue_z (* (`GameplayStatics.GetWorldDeltaSeconds`) (`self.speed`))))))

(fn `UserConstructionScript`)