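; Boss_Fire_BP is a short-lived boss fire hazard that damages the player character and destroys itself two seconds after spawning.
; Tick runs a small multi-sphere trace at the actor's location, matches hits by "MyCharacter" display name, then applies damage to the MyCharacter instance.
; The trailing Delay in Tick does not throttle this, so damage can land every frame, once per matching hit.
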(event `self.ReceiveBeginPlay`
  (`KismetSystemLibrary.Delay` 2.0)
  (`self.K2_DestroyActor`))

(event `self.ReceiveTick`
  (params (DeltaSeconds :type "Float (single-precision)"))
  (`self.Apply_Damage`)
  (`KismetSystemLibrary.Delay` 0.8))

(fn `Apply_Damage`
  (bind _returnvalue (`self.K2_GetActorLocation`))
  (bind _outhits (`KismetSystemLibrary.SphereTraceMulti` _returnvalue _returnvalue 10.0 "TraceTypeQuery1"))
  (for _array_element _outhits
    (if (`KismetStringLibrary.Contains` (`KismetSystemLibrary.GetDisplayName` (`.HitActor` (`GameplayStatics.BreakHitResult` _array_element))) "MyCharacter")
      (bind _returnvalue_2 (`GameplayStatics.GetActorOfClass` "/Game/Logical_And_/Blueprints/Actors/Player/MyCharacter.MyCharacter_C"))
      (`GameplayStatics.ApplyDamage` _returnvalue_2 (`self.Damage`)))))

(fn `UserConstructionScript`)