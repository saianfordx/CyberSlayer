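; Torch_01_BP is a boss-area torch actor, a child Blueprint that tunes behavior inherited from its parent.
; On BeginPlay it sets its MaxZ limit and Speed, then runs the parent's BeginPlay.
; Tick, construction and Adjust_Position only call the parent versions, so any positioning logic lives in the parent class.
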(event `self.ReceiveBeginPlay`
  (set `self.max_z` -160.0)
  (set `self.speed` 10.0)
  (`parent.ReceiveBeginPlay`))

(event `self.ReceiveTick`
  (params (DeltaSeconds :type "Float (single-precision)"))
  (`parent.ReceiveTick` DeltaSeconds))

(fn `Adjust_Position`
  (`parent.Adjust_Position`))

(fn `UserConstructionScript`
  (`parent.UserConstructionScript`))