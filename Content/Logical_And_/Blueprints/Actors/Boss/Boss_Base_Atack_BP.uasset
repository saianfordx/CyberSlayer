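; Base boss attack projectile that falls straight down, damaging the player character and spawning an explosion on contact.
; Each Tick moves it down by Speed, then runs a small sphere trace that identifies the player by a "MyCharacter" display-name substring.
; It destroys itself on hit, at a low Z limit, or when the Boss_BP found in the level has no life left.
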(event `self.ReceiveBeginPlay`)

(event `self.ReceiveTick`
  (params (DeltaSeconds :type "Float (single-precision)"))
  (`self.Check_Life`)
  (`self.Movement`)
  (`self.Apply_Damage`)
  (`self.Destroy_Actor`))

(fn `Apply_Damage`
  (bind _returnvalue (`self.K2_GetActorLocation`))
  (bind _outhits (`KismetSystemLibrary.SphereTraceMulti` _returnvalue _returnvalue 5.0 "TraceTypeQuery1"))
  (for _array_element _outhits
    (if (`KismetStringLibrary.Contains` (`KismetSystemLibrary.GetDisplayName` (`.HitActor` (`GameplayStatics.BreakHitResult` _array_element))) "MyCharacter")
      (bind _returnvalue_2 (`GameplayStatics.GetActorOfClass` "/Game/Logical_And_/Blueprints/Actors/Player/MyCharacter.MyCharacter_C"))
      (`GameplayStatics.ApplyDamage` _returnvalue_2 (`self.Damage`))
      (`|SpawnActorFromClass` "/Game/Logical_And_/Blueprints/Animations/Explotions/Explotion_01/Explotion_01_BP.Explotion_01_BP_C" (`self.GetTransform`) "Undefined" "OverrideRootScale" null null)
      (`self.K2_DestroyActor`))))

(fn `Check_Life`
  (bind _returnvalue (`GameplayStatics.GetActorOfClass` "/Game/Logical_And_/Blueprints/Actors/Boss/Boss_BP.Boss_BP_C"))
  (bind _asboss_bp (cast `/Game/Logical_And_/Blueprints/Actors/Boss/Boss_BP` _returnvalue))
  (bind _currentlife (`/Game/Logical_And_/Blueprints/Actors/Boss/Boss_BP.Get_Current_Life` _asboss_bp))
  (if (<= _currentlife 0.0)
    (`self.K2_DestroyActor`)))

(fn `Destroy_Actor`
  (bind (_returnvalue_x _returnvalue_y _returnvalue_z) (`KismetMathLibrary.BreakVector` (`self.K2_GetActorLocation`)))
  (if (<= _returnvalue_z -500.0)
    (`self.K2_DestroyActor`)))

(fn `Movement`
  (bind (_returnvalue_x _returnvalue_y _returnvalue_z) (`KismetMathLibrary.BreakVector` (`SceneComponent.K2_GetComponentLocation` (`self.DefaultSceneRoot`))))
  (`self.K2_SetActorLocation` (`KismetMathLibrary.MakeVector` _returnvalue_x _returnvalue_y (- _returnvalue_z (* (`GameplayStatics.GetWorldDeltaSeconds`) (`self.Speed`))))))

(fn `UserConstructionScript`)