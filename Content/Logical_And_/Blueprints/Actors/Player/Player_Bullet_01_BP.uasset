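; Player bullet that flies along world X in the direction set by IsForward, turning to face backward on BeginPlay when needed.
; Each Tick moves it by Speed, then runs a sphere trace at its location and identifies Enemy or Boss_BP hits by display name.
; Damage goes to the first GetActorOfClass result rather than the hit actor reference, then the bullet spawns an explosion and destroys itself.
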(event `self.ReceiveBeginPlay`
  (`self.LookAt`))

(event `self.ReceiveTick`
  (params (DeltaSeconds :type "Float (single-precision)"))
  (`self.Shoot`)
  (`self.ApplyDamage`))

(fn `ApplyDamage`
  (bind _returnvalue (`self.K2_GetActorLocation`))
  (bind _outhits (`KismetSystemLibrary.SphereTraceMulti` _returnvalue _returnvalue 25.0 "TraceTypeQuery1"))
  (for _array_element _outhits
    (bind (_bblockinghit _binitialoverlap _time _distance _location _impactpoint _normal _impactnormal _physmat _hitactor) (`GameplayStatics.BreakHitResult` _array_element))
    (bind _returnvalue_2 (`KismetSystemLibrary.GetDisplayName` _hitactor))
    (if (`KismetStringLibrary.Contains` _returnvalue_2 "Enemy")
      (bind _returnvalue_3 (`GameplayStatics.GetActorOfClass` (`GameplayStatics.GetObjectClass` _hitactor)))
      (bind _asenemy (cast `/Game/Logical_And_/Blueprints/Actors/Enemy` _returnvalue_3))
      (`/Game/Logical_And_/Blueprints/Actors/Enemy.SelfApplyDamage` _asenemy (`self.Damage`))
      (`|SpawnActorFromClass` "/Game/Logical_And_/Blueprints/Animations/Explotions/Explotion_01/Explotion_01_BP.Explotion_01_BP_C" (`self.GetTransform`) "Undefined" "OverrideRootScale" null null :!label _label)
      (`self.K2_DestroyActor`)
      (elif (`KismetStringLibrary.Contains` _returnvalue_2 "Boss_BP")
        (bind _returnvalue_4 (`GameplayStatics.GetActorOfClass` "/Game/Logical_And_/Blueprints/Actors/Boss/Boss_BP.Boss_BP_C"))
        (bind _asboss_bp (cast `/Game/Logical_And_/Blueprints/Actors/Boss/Boss_BP` _returnvalue_4))
        (`/Game/Logical_And_/Blueprints/Actors/Boss/Boss_BP.Self_Apply_Damage` _asboss_bp (`self.Damage`))
        (goto _label)))))

(fn `GetImpactPoint`
  (returns (TargetPoint :type "Vector Structure"))
  (bind _returnvalue (`GameplayStatics.GetActorOfClass` "/Game/Migrations/2DSideScrollerBP/Semana_05/2DSideScrollerBP/Blueprints/MyCharacter.MyCharacter_C"))
  (bind (_returnvalue_x _returnvalue_y _returnvalue_z) (`KismetMathLibrary.BreakVector` (`self.K2_GetActorLocation` _returnvalue)))
  (return (`KismetMathLibrary.Normal` (`KismetMathLibrary.MakeVector` (+ _returnvalue_x 500.0) _returnvalue_y _returnvalue_z))))

(fn `LookAt`
  (if (not (`self.isForward`))
    (`self.K2_SetActorRotation` (`KismetMathLibrary.MakeRotator` 0.0 0.0 180.0))))

(fn `SetIsForward`
  (params (NewParam :type Boolean))
  (set `self.isForward` NewParam))

(fn `Shoot`
  (bind (_returnvalue_x _returnvalue_y _returnvalue_z) (`KismetMathLibrary.BreakVector` (`self.K2_GetActorLocation`)))
  (bind (_returnvalue_x_2 _returnvalue_y_2 _returnvalue_z_2) (`KismetMathLibrary.BreakVector` (`self.K2_GetActorLocation`)))
  (if (`self.isForward`)
    (`self.K2_SetActorLocation` (`KismetMathLibrary.MakeVector` (+ (* (`self.Speed`) (`GameplayStatics.GetWorldDeltaSeconds`)) _returnvalue_x_2) _returnvalue_y_2 _returnvalue_z_2))
    (else
      (`self.K2_SetActorLocation` (`KismetMathLibrary.MakeVector` (- _returnvalue_x (* (`self.Speed`) (`GameplayStatics.GetWorldDeltaSeconds`))) _returnvalue_y _returnvalue_z)))))

(fn `UserConstructionScript`)