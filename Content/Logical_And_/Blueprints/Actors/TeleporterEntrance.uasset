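; TeleporterEntrance is a level-exit actor that opens Level_02 when the player character comes within a small radius.
; Every Tick it calls Teleport, which runs a zero-length multi sphere trace on the Visibility channel at its location and matches hit actors by "MyCharacter" in the display name.
; Disconnected nodes in Teleport would instead move the hit actor to the TeleporterExit's location, but they never run.
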(event `self.ReceiveTick`
  (params (DeltaSeconds :type "Float (single-precision)"))
  (`self.Teleport`))

(fn `Teleport`
  (bind _returnvalue (`self.K2_GetActorLocation`))
  (bind _outhits (`KismetSystemLibrary.SphereTraceMulti` _returnvalue _returnvalue 50.0 "TraceTypeQuery1"))
  (for _array_element _outhits
    (if (`KismetStringLibrary.Contains` (`KismetSystemLibrary.GetDisplayName` (`.HitActor` (`GameplayStatics.BreakHitResult` _array_element))) "MyCharacter")
      (`GameplayStatics.OpenLevelBySoftObjectPtr` "/Game/2DSideScrollerBP/Levels/Level_02.Level_02"))))

(fn `UserConstructionScript`)